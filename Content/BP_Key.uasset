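; BP_Key is an interactable key that records its KeyNumber in MyGameMode when used.
; BeginPlay caches the game mode, and Interact overwrites its Keys value with KeyNumber, then prints the acquired key's name and a "Hello" string.
; The construction script colors the Sphere green or red from KeyNumber.
; The actor stays in the world after interaction.
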(event `self.ReceiveBeginPlay`
  (bind _asmy_game_mode (cast `/Game/ThirdPerson/Blueprints/MyGameMode` (`GameplayStatics.GetGameMode`)))
  (set `self.My_GM` _asmy_game_mode))

(event `/Game/BPI_Interactable.Interact`
  (bind _output_get (set `/Game/ThirdPerson/Blueprints/MyGameMode.Keys` (`self.KeyNumber`) (`self.My_GM`)))
  (`KismetSystemLibrary.PrintString` (`KismetStringLibrary.Concat_StrStr` "Key" (`|GetArrayItem` (`self.Names`) _output_get) "Acquired"))
  (`KismetSystemLibrary.PrintString` "Hello"))

(fn `UserConstructionScript`
  (bind _sphere (`self.Sphere`))
  (switch `int` (`self.KeyNumber`)
    (:`0`
      (`PrimitiveComponent.SetMaterial` _sphere 0 "/Game/MI_Green.MI_Green"))
    (:`1`
      (`PrimitiveComponent.SetMaterial` _sphere 0 "/Game/MI_Red.MI_Red"))))