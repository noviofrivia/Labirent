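; BP_MazeCell is one maze tile that builds its floor, flagged walls, optional point light and chosen spike, axe or gas trap.
; The construction script scales meshes from grid size and wall height, and sets the trap's child actor class.
; On BeginPlay, trap-free cells randomly spawn gold or another actor.
; The cell binds to the player's maze gate dispatcher, recoloring its light to the player's color when IsInside is false.
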(event `self.ReceiveBeginPlay`
  (bind _returnvalue (`SceneComponent.K2_GetComponentLocation` (`self.Scene`)))
  (bind _asmy_game_mode (cast `/Game/ThirdPerson/Blueprints/MyGameMode` (`GameplayStatics.GetGameMode`)))
  (bind _output_get (set `self.My_GM` _asmy_game_mode))
  (set `self.New Light Color` (`/Game/ThirdPerson/Blueprints/MyGameMode.LightColor` _output_get))
  (bind _asbp_third_person_character (cast `/Game/BP_ThirdPersonCharacter` (`GameplayStatics.GetPlayerCharacter` 0)))
  (set `self.Player` _asbp_third_person_character)
  (add `/Game/BP_ThirdPersonCharacter.DP_MazeGate` _asbp_third_person_character (delegate `MazeGate_Event`))
  (if (`self.Trap`)
    _
    (elif (> (`KismetMathLibrary.RandomIntegerInRange` 0 10) 9)
      (`|SpawnActorFromClass` "/Game/BP_Medkit.BP_Medkit_C" (`KismetMathLibrary.MakeTransform` _returnvalue) "Undefined" "MultiplyWithRoot" null null)
      (elif (> (`KismetMathLibrary.RandomIntegerInRange` 0 10) 7)
        (`|SpawnActorFromClass` "/Game/BP_Gold.BP_Gold_C" (`KismetMathLibrary.MakeTransform` (- _returnvalue (0.0 0.0 50.0))) "Undefined" "MultiplyWithRoot" null null)))))

(event `MazeGate_Event`
  (params (`IsInside?` :type Boolean))
  (bind _pointlight (`self.PointLight`))
  (if (not `IsInside?`)
    (`/Engine/EditorBlueprintResources/StandardMacros.IsValid` _pointlight
      (:`Is Valid`
        (`LightComponent.SetLightColor` _pointlight (`/Game/BP_ThirdPersonCharacter.LightColor` (`self.Player`)) true)))))

(fn `UserConstructionScript`
  (locals (WallLength :type "Float (double-precision)") (WallThickness :type "Float (double-precision)"))
  (bind _gridsize (`self.GridSize`))
  (bind _walllength (`local.WallLength`))
  (bind _wallheight (`self.WallHeight`))
  (bind _returnvalue (/ _wallheight 2.0))
  (set `local.WallLength` _gridsize)
  (set `local.WallThickness` (* _gridsize 0.1))
  (`SceneComponent.SetRelativeScale3D` (`self.Floor`) (`self.CubeSizeToScale` (`KismetMathLibrary.MakeVector` _walllength _walllength (`local.WallThickness`))))
  (if (`self.WestWall`)
    (`AddComponent|NODE_AddStaticMeshComponent-2` :`RelativeTransform` (`KismetMathLibrary.MakeTransform` (0.0 0.0 0.0) (struct) (`self.CubeSizeToScale` (`KismetMathLibrary.MakeVector` (`local.WallLength`) (`local.WallThickness`) (`self.WallHeight`))))))
  (if (`self.SouthWall`)
    (`AddComponent|NODE_AddStaticMeshComponent-3` :`RelativeTransform` (`KismetMathLibrary.MakeTransform` (0.0 0.0 0.0) (struct) (`self.CubeSizeToScale` (`KismetMathLibrary.MakeVector` (`local.WallThickness`) (`local.WallLength`) (`self.WallHeight`))))))
  (if (`self.EastWall`)
    (`AddComponent|NODE_AddStaticMeshComponent-0` :`RelativeTransform` (`KismetMathLibrary.MakeTransform` (`KismetMathLibrary.MakeVector` 0.0 (- (`local.WallLength`) (`local.WallThickness`))) (struct) (`self.CubeSizeToScale` (`KismetMathLibrary.MakeVector` (`local.WallLength`) (`local.WallThickness`) (`self.WallHeight`))))))
  (if (`self.NorthWall`)
    (`AddComponent|NODE_AddStaticMeshComponent-1` :`RelativeTransform` (`KismetMathLibrary.MakeTransform` (`KismetMathLibrary.MakeVector` (- (`local.WallLength`) (`local.WallThickness`))) (struct) (`self.CubeSizeToScale` (`KismetMathLibrary.MakeVector` (`local.WallThickness`) (`local.WallLength`) (`self.WallHeight`))))))
  (if (`self.Light`)
    (bind _returnvalue_2 (`AddComponent|NODE_AddPointLightComponent-0` :`RelativeTransform` (`KismetMathLibrary.MakeTransform` (`KismetMathLibrary.MakeVector` _returnvalue _returnvalue _wallheight))))
    (bind _output_get (set `self.PointLight` _returnvalue_2))
    (`LightComponent.SetIntensity` _output_get 5000.0)
    (`LightComponent.SetLightColor` _output_get (`self.New Light Color`) true))
  (switch `/Game/TrapType` (`self.TrapType`)
    (:`NewEnumerator0`
      (set `self.Trap` false))
    (:`NewEnumerator1`
      (set `self.Trap` true)
      (`ChildActorComponent.SetChildActorClass` (`self.ChildActor`) "/Game/BP_TrapSpike.BP_TrapSpike_C"))
    (:`NewEnumerator2`
      (set `self.Trap` true)
      (`ChildActorComponent.SetChildActorClass` (`self.ChildActor`) "/Game/BP_TrapAxe.BP_TrapAxe_C")
      (`SceneComponent.K2_SetWorldRotation` (`self.ChildActor`) (struct :`Yaw` 270.0) false false))
    (:`NewEnumerator3`
      (set `self.Trap` true)
      (`ChildActorComponent.SetChildActorClass` (`self.ChildActor`) "/Game/BP_TrapGas.BP_TrapGas_C"))))