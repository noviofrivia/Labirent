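; BP_Switch is an interactable switch tied to a TrapType enum value, used to turn off traps of that type.
; On BeginPlay it caches the player's BP_ThirdPersonCharacter and displays the enum name on its TextRender.
; Interact passes TrapType to the player's CallDPTrap, so the trap call is routed through the character, then prints a message saying that trap was turned off.
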(event `self.ReceiveBeginPlay`
  (bind _asbp_third_person_character (cast `/Game/BP_ThirdPersonCharacter` (`GameplayStatics.GetPlayerCharacter` 0)))
  (set `self.Player` _asbp_third_person_character)
  (`TextRenderComponent.K2_SetText` (`self.TextRender`) (`KismetTextLibrary.Conv_StringToText` (`|GetEnumeratorNameAsString` (`self.TrapType`)))))

(event `/Game/BPI_Interactable.Interact`
  (bind _traptype (`self.TrapType`))
  (`/Game/BP_ThirdPersonCharacter.DP_Trap` (`self.Player`) _traptype)
  (`KismetSystemLibrary.PrintString` (`KismetStringLibrary.Concat_StrStr` "Turned off trap: " (`|GetEnumeratorNameAsString` _traptype))))

(fn `UserConstructionScript`)