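; Gold pickup worth a random amount, shown on its text render when play begins.
; Construction script rolls the value and runs a CreateMesh macro against three thresholds, so richer piles get more meshes, each with random XY offset and scale.
; Interact adds the value to PlayerGold on MyGameMode, prints the new total and destroys the actor.
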(event `self.ReceiveBeginPlay`
  (bind _asmy_game_mode (cast `/Game/ThirdPerson/Blueprints/MyGameMode` (`GameplayStatics.GetGameMode`)))
  (set `self.My_GM` _asmy_game_mode)
  (`TextRenderComponent.K2_SetText` (`self.TextRender`) (`KismetTextLibrary.Conv_IntToText` (`self.ItemGold`))))

(event `/Game/BPI_Interactable.Interact`
  (bind _output_get (set `/Game/ThirdPerson/Blueprints/MyGameMode.PlayerGold` (+ (`/Game/ThirdPerson/Blueprints/MyGameMode.PlayerGold` (`self.My_GM`)) (`self.ItemGold`)) (`self.My_GM`)))
  (`KismetSystemLibrary.PrintString` (`KismetStringLibrary.Concat_StrStr` "Current Gold" (`KismetStringLibrary.Conv_IntToString` _output_get)))
  (`self.K2_DestroyActor`))

(fn `UserConstructionScript`
  (bind _itemgold (`self.ItemGold`))
  (set `self.ItemGold` (`KismetMathLibrary.RandomIntegerInRange` 1 99))
  (`self.create_mesh` (>= _itemgold 76)
    (:`then`
      _)
    (:`false`
      _))
  (`self.create_mesh` (>= _itemgold 26)
    (:`then`
      _)
    (:`false`
      _))
  (`self.create_mesh` (>= _itemgold 1)))