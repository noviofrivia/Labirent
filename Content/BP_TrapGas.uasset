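; BP_TrapGas is a gas trap that deals damage over time to the player while they stay inside its DamageBox.
; Box overlaps start and clear a looping DOT timer that calls the player's HealthUpdate at a set interval.
; On BeginPlay it binds to the player character's trap dispatcher, and a matching TrapType event disables DamageBox collision and destroys the Gas component.
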(event `self.ReceiveBeginPlay`
  (bind _asbp_third_person_character (cast `/Game/BP_ThirdPersonCharacter` (`GameplayStatics.GetPlayerCharacter` 0)))
  (bind _output_get (set `self.Player` _asbp_third_person_character))
  (add `/Game/BP_ThirdPersonCharacter.DP_Trap` _output_get (delegate `DP_TrapEvent`)))

(event `DP_TrapEvent`
  (params (TrapType :type "/Game/TrapType Enum" :default "NewEnumerator0"))
  (if (`|EnumEquality` TrapType (`self.TrapType`))
    (`PrimitiveComponent.SetCollisionEnabled` (`self.DamageBox`) "NoCollision")
    (`ActorComponent.K2_DestroyComponent` (`self.Gas`))))

(event `self.DamageBox.OnComponentBeginOverlap`
  (params (OverlappedComponent :type "PrimitiveComponent Object Reference") (OtherActor :type "Actor Object Reference") (OtherComp :type "PrimitiveComponent Object Reference") (OtherBodyIndex :type Integer) (bFromSweep :type Boolean) (SweepResult :type "HitResult Structure (by ref)"))
  (if (== OtherActor (`self.Player`))
    (`KismetSystemLibrary.K2_SetTimer` null "DOT" (`self.DOT_Time`) true)))

(event `DOT`
  (`/Game/BP_ThirdPersonCharacter.HealthUpdate` (`self.Player`) (`self.DOT_Damage`)))

(event `self.DamageBox.OnComponentEndOverlap`
  (params (OverlappedComponent :type "PrimitiveComponent Object Reference") (OtherActor :type "Actor Object Reference") (OtherComp :type "PrimitiveComponent Object Reference") (OtherBodyIndex :type Integer))
  (if (== OtherActor (`self.Player`))
    (`KismetSystemLibrary.K2_ClearTimer` null "DOT")))

(fn `UserConstructionScript`)