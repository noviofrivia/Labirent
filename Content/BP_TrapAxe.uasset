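; BP_TrapAxe is an axe trap that swings and damages the player.
; When the player overlaps ActivasionMesh, that mesh is destroyed and the AxeTL timeline plays, driving the axe's roll.
; DamageBox overlaps reduce the player's health through HealthUpdate.
; A trap event bound on the player character disarms a matching TrapType by resetting the axe rotation, disabling damage collision and destroying the timeline.
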(event `self.ReceiveBeginPlay`
  (bind _asbp_third_person_character (cast `/Game/BP_ThirdPersonCharacter` (`GameplayStatics.GetPlayerCharacter` 0)))
  (bind _output_get (set `self.Player` _asbp_third_person_character))
  (add `/Game/BP_ThirdPersonCharacter.DP_Trap` _output_get (delegate `DP_TrapEvent`)))

(event `DP_TrapEvent`
  (params (TrapType :type "/Game/TrapType Enum" :default "NewEnumerator0"))
  (if (`|EnumEquality` TrapType (`self.TrapType`))
    (`KismetSystemLibrary.PrintString` "Hello")
    (`SceneComponent.K2_SetRelativeRotation` (`self.Axe`) (struct :`Pitch` 180.0) false false)
    (`PrimitiveComponent.SetCollisionEnabled` (`self.DamageBox`) "NoCollision")
    (`ActorComponent.K2_DestroyComponent` (`self.AxeTL`))))

(event `self.DamageBox.OnComponentBeginOverlap`
  (params (OverlappedComponent :type "PrimitiveComponent Object Reference") (OtherActor :type "Actor Object Reference") (OtherComp :type "PrimitiveComponent Object Reference") (OtherBodyIndex :type Integer) (bFromSweep :type Boolean) (SweepResult :type "HitResult Structure (by ref)"))
  (if (== OtherActor (`self.Player`))
    (`/Game/BP_ThirdPersonCharacter.HealthUpdate` (`self.Player`) -15.0)))

(event `self.ActivasionMesh.OnComponentBeginOverlap`
  (params (OverlappedComponent :type "PrimitiveComponent Object Reference") (OtherActor :type "Actor Object Reference") (OtherComp :type "PrimitiveComponent Object Reference") (OtherBodyIndex :type Integer) (bFromSweep :type Boolean) (SweepResult :type "HitResult Structure (by ref)"))
  (if (== OtherActor (`self.Player`))
    (`ActorComponent.K2_DestroyComponent` (`self.ActivasionMesh`))
    (`self.AxeTL`
      (:`then`
        (bind (_direction _newtrack_0) (`Timeline|AxeTL`)
          (:`Update`
            (`SceneComponent.K2_SetRelativeRotation` (`self.Axe`) (`KismetMathLibrary.MakeRotator` _newtrack_0 180.0) false false))))
      (:`else`))))

(fn `UserConstructionScript`)