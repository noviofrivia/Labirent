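; BP_SlidingDoor is a key-gated door that slides open on interaction.
; It caches MyGameMode at BeginPlay and, on Interact, opens only when the game mode's Keys value exactly equals its KeyNumber, otherwise printing a message.
; Despite its name, the DoorRotate timeline translates the mesh, lerping its relative location from StartLoc to FinishLoc.
; The construction script colors the door green or red from KeyNumber.
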(event `self.ReceiveBeginPlay`
  (bind _asmy_game_mode (cast `/Game/ThirdPerson/Blueprints/MyGameMode` (`GameplayStatics.GetGameMode`)))
  (set `self.My_GM` _asmy_game_mode))

(event `/Game/BPI_Interactable.Interact`
  (if (== (`/Game/ThirdPerson/Blueprints/MyGameMode.Keys` (`self.My_GM`)) (`self.KeyNumber`))
    (bind (_direction _newtrack_0) (`Timeline|DoorRotate`)
      (:`Update`
        (`SceneComponent.K2_SetRelativeLocation` (`self.SM_Door`) (`KismetMathLibrary.VLerp` (`self.StartLoc`) (`self.FinishLoc`) _newtrack_0) false false)))
    (else
      (`KismetSystemLibrary.PrintString` "You don't have the correct key"))))

(fn `UserConstructionScript`
  (bind _sm_door (`self.SM_Door`))
  (switch `int` (`self.KeyNumber`)
    (:`0`
      (`PrimitiveComponent.SetMaterial` _sm_door 0 "/Game/MI_Green.MI_Green"))
    (:`1`
      (`PrimitiveComponent.SetMaterial` _sm_door 0 "/Game/MI_Red.MI_Red"))))