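; BP_Checkpoint is a checkpoint that records the player's position as a spawn location when interacted with.
; On BeginPlay it caches the third-person player character and the custom game instance.
; Its Interact event writes the player's current location, rather than the checkpoint's, to SpawnLoc on the game instance and prints a confirmation.
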(event `self.ReceiveBeginPlay`
  (bind _asbp_third_person_character (cast `/Game/BP_ThirdPersonCharacter` (`GameplayStatics.GetPlayerCharacter` 0)))
  (set `self.Player` _asbp_third_person_character)
  (bind _asmy_game_instance (cast `/Game/MyGameInstance` (`GameplayStatics.GetGameInstance`)))
  (set `self.MyGameInstance` _asmy_game_instance))

(event `/Game/BPI_Interactable.Interact`
  (set `/Game/MyGameInstance.SpawnLoc` (`self.K2_GetActorLocation` (`self.Player`)) (`self.MyGameInstance`))
  (`KismetSystemLibrary.PrintString` "Checkpoint saved"))

(fn `UserConstructionScript`)